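; GridImpl is a grid actor Blueprint that currently serves to visualize its bounding sphere for debugging.
; Each Tick, it transforms BoundingSphereCenter by the actor transform, draws a debug sphere of BoundingSphereRadius there and prints that world position.
; An unconnected leftover chain would scale ShieldBubble uniformly from the largest axis of the actor's bounds extent, but never runs.
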(event `self.ReceiveBeginPlay`)

(event `self.ReceiveActorBeginOverlap`
  (params (OtherActor :type "Actor Object Reference")))

(event `self.ReceiveTick`
  (params (DeltaSeconds :type "Float (single-precision)"))
  (bind _returnvalue (`KismetMathLibrary.TransformLocation` (`self.GetTransform`) (`self.BoundingSphereCenter`)))
  (`KismetSystemLibrary.DrawDebugSphere` _returnvalue (`self.BoundingSphereRadius`) 12 (struct :`G` 0.114498 :`B` 1.0 :`A` 1.0) 1.0)
  (`KismetSystemLibrary.PrintString` (`KismetStringLibrary.Conv_VectorToString` _returnvalue)))

(fn `UserConstructionScript`)