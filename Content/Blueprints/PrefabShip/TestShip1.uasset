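; TestShip1 is a prefab test ship Blueprint that assembles a fixed ship layout on a part grid.
; On BeginPlay it calls CreateAndAddToGrid for each part at hard-coded grid coordinates.
; The layout combines armor, thrusters, an engine, cannon and turret weapons, a command center and fusion reactors.
; There is no other logic; overlap, tick and construction script are empty.
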(event `self.ReceiveBeginPlay`
  (`self.CreateAndAddToGrid` "/Game/Blueprints/Part/BasicArmor.BasicArmor_C")
  (`self.CreateAndAddToGrid` "/Game/Blueprints/Part/BasicArmor.BasicArmor_C" 1)
  (`self.CreateAndAddToGrid` "/Game/Blueprints/Part/BasicArmor.BasicArmor_C" -1)
  (`self.CreateAndAddToGrid` "/Game/Blueprints/Part/Thruster.Thruster_C" -2)
  (`self.CreateAndAddToGrid` "/Game/Blueprints/Part/Thruster.Thruster_C" 2)
  (`self.CreateAndAddToGrid` "/Game/Blueprints/Part/Engine.Engine_C" -2 1)
  (`self.CreateAndAddToGrid` "/Game/Blueprints/Part/BoltCannon.BoltCannon_C" 3)
  (`self.CreateAndAddToGrid` "/Game/Blueprints/Part/BoltTurret.BoltTurret_C" 3 -1)
  (`self.CreateAndAddToGrid` "/Game/Blueprints/Part/PlasmaCannon.PlasmaCannon_C" 3 1)
  (`self.CreateAndAddToGrid` "/Game/Blueprints/Part/CommandCenter.CommandCenter_C" -3)
  (`self.CreateAndAddToGrid` "/Game/Blueprints/Part/FusionReactor.FusionReactor_C" -4)
  (`self.CreateAndAddToGrid` "/Game/Blueprints/Part/FusionReactor.FusionReactor_C" -4 1))

(event `self.ReceiveActorBeginOverlap`
  (params (OtherActor :type "Actor Object Reference")))

(event `self.ReceiveTick`
  (params (DeltaSeconds :type "Float (single-precision)")))

(fn `UserConstructionScript`)