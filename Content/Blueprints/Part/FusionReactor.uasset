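; FusionReactor is a part actor whose cube mesh visually reflects the power level of the grid it is attached to.
; On BeginPlay it creates a dynamic material instance from the FusionReactor material and assigns it to the cube.
; Each tick it casts the owner of the cube's attach parent to GridImpl and writes that grid's power percentage into the material's PowerLevel parameter.
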(event `self.ReceiveBeginPlay`
  (bind _returnvalue (`KismetMaterialLibrary.CreateDynamicMaterialInstance` "/Game/Materials/FusionReactor.FusionReactor"))
  (`PrimitiveComponent.SetMaterial` (`self.Cube`) 0 _returnvalue)
  (set `self.Mat` _returnvalue))

(event `self.ReceiveActorBeginOverlap`
  (params (OtherActor :type "Actor Object Reference")))

(event `self.ReceiveTick`
  (params (DeltaSeconds :type "Float (single-precision)"))
  (bind _asgrid_impl (cast `/Game/Blueprints/GridImpl` (`ActorComponent.GetOwner` (`SceneComponent.GetAttachParent` (`self.Cube`)))))
  (`MaterialInstanceDynamic.SetScalarParameterValue` (`self.Mat`) "PowerLevel" (`Grid.GetPowerPct` _asgrid_impl)))

(fn `UserConstructionScript`)